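; BP_Locker is a locker the player can hide in, with a key prompt widget shown while the character overlaps its trigger.
; HidePlayer stores the player, toggles hiding and replays a timeline that swings the door's yaw.
; ToggleHide flips the player's visibility and blends the camera between the locker and the player.
; The trigger only manages the prompt, so HidePlayer must be called from outside this graph.
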(event `AnimateDoor`
  (bind (_direction _doortrack) (`Timeline|ToggleDoor` :!via `PlayFromStart`)
    (:`Update`
      (`SceneComponent.K2_SetRelativeRotation` (`self.Door`) (`KismetMathLibrary.MakeRotator` 0.0 0.0 (`KismetMathLibrary.Lerp` 0.0 90.0 _doortrack)) false false))))

(event `HidePlayer`
  (params (Player :type "/Game/ThirdPerson/Blueprints/BP_ThirdPersonCharacter Object Reference"))
  (set `self.PlayerRef` Player)
  (`|ExecutionSequence`
    (:`then_0`
      (`self.ToggleHide`))
    (:`then_1`
      (`self.AnimateDoor`))))

(event `self.EnterTrigger.OnComponentBeginOverlap`
  (params (OverlappedComponent :type "PrimitiveComponent Object Reference") (OtherActor :type "Actor Object Reference") (OtherComp :type "PrimitiveComponent Object Reference") (OtherBodyIndex :type Integer) (bFromSweep :type Boolean) (SweepResult :type "HitResult Structure (by ref)"))
  (cast `/Game/ThirdPerson/Blueprints/BP_ThirdPersonCharacter` OtherActor)
  (bind _returnvalue (`|CreateWidget` "/Game/BPs/BP_DisplayKey.BP_DisplayKey_C"))
  (bind _output_get (set `self.KeyDisplay` _returnvalue))
  (`UserWidget.AddToViewport` _output_get 0))

(event `self.EnterTrigger.OnComponentEndOverlap`
  (params (OverlappedComponent :type "PrimitiveComponent Object Reference") (OtherActor :type "Actor Object Reference") (OtherComp :type "PrimitiveComponent Object Reference") (OtherBodyIndex :type Integer))
  (cast `/Game/ThirdPerson/Blueprints/BP_ThirdPersonCharacter` OtherActor)
  (`Widget.RemoveFromParent` (`self.KeyDisplay`)))

(fn `ToggleHide`
  (bind _returnvalue (`GameplayStatics.GetPlayerController` 0))
  (bind _playerref (`self.PlayerRef`))
  (if (`self.IsHiding`)
    (set `self.IsHiding` false)
    (`self.SetActorHiddenInGame` _playerref false)
    (`PlayerController.SetViewTargetWithBlend` _returnvalue _playerref 0.5 "VTBlend_Linear" 0.0 false)
    (else
      (set `self.IsHiding` true)
      (`self.SetActorHiddenInGame` _playerref true)
      (`PlayerController.SetViewTargetWithBlend` _returnvalue self 0.5 "VTBlend_Linear" 0.0 false))))

(fn `UserConstructionScript`)
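; Inventory component for the third-person character that stores items in an array and notifies the on-screen inventory widget of changes.
; Adding appends the item, then casts the owner to BP_ThirdPersonCharacter and passes the item to its InventoryWidget through AddItemToUI.
; Removal takes no argument: on a non-empty array it removes by the last entry's value, then calls the same AddItemToUI with an empty string.
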(fn `AddItemToInventory`
  (params (NewItem :type "String (by ref)"))
  (`KismetArrayLibrary.Array_Add` (`self.Inventory`) NewItem)
  (bind _asbp_third_person_character (cast `/Game/ThirdPerson/Blueprints/BP_ThirdPersonCharacter` (`self.GetOwner`)))
  (`/Game/BPs/Inventory/B_InventoryWidget.AddItemToUI` (`/Game/ThirdPerson/Blueprints/BP_ThirdPersonCharacter.InventoryWidget` _asbp_third_person_character) NewItem))

(fn `RemoveItemFromInventory`
  (bind _inventory (`self.Inventory`))
  (if (> (`KismetArrayLibrary.Array_Length` (`self.Inventory`)) 0)
    (`KismetArrayLibrary.Array_RemoveItem` _inventory (`|GetArrayItem` _inventory (`KismetArrayLibrary.Array_LastIndex` _inventory)))
    (bind _asbp_third_person_character (cast `/Game/ThirdPerson/Blueprints/BP_ThirdPersonCharacter` (`self.GetOwner`)))
    (`/Game/BPs/Inventory/B_InventoryWidget.AddItemToUI` (`/Game/ThirdPerson/Blueprints/BP_ThirdPersonCharacter.InventoryWidget` _asbp_third_person_character) "")))
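; BP_VHS is a pickup item actor, named as a VHS, that shows a key prompt when the player character is near.
; Its Trigger overlap creates and displays a BP_DisplayKey widget for BP_ThirdPersonCharacter, and removes it when the overlap ends.
; PickupItem prints a message, starts destruction through a short-delay event, and returns the Item to its caller.
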(event `Destroy item`
  (`KismetSystemLibrary.Delay` 0.1)
  (`self.K2_DestroyActor`))

(event `self.Trigger.OnComponentBeginOverlap`
  (params (OverlappedComponent :type "PrimitiveComponent Object Reference") (OtherActor :type "Actor Object Reference") (OtherComp :type "PrimitiveComponent Object Reference") (OtherBodyIndex :type Integer) (bFromSweep :type Boolean) (SweepResult :type "HitResult Structure (by ref)"))
  (cast `/Game/ThirdPerson/Blueprints/BP_ThirdPersonCharacter` OtherActor)
  (bind _returnvalue (`|CreateWidget` "/Game/BPs/BP_DisplayKey.BP_DisplayKey_C"))
  (bind _output_get (set `self.KeyDisplay` _returnvalue))
  (`UserWidget.AddToViewport` _output_get 0))

(event `self.Trigger.OnComponentEndOverlap`
  (params (OverlappedComponent :type "PrimitiveComponent Object Reference") (OtherActor :type "Actor Object Reference") (OtherComp :type "PrimitiveComponent Object Reference") (OtherBodyIndex :type Integer))
  (cast `/Game/ThirdPerson/Blueprints/BP_ThirdPersonCharacter` OtherActor)
  (`Widget.RemoveFromParent` (`self.KeyDisplay`)))

(fn `PickupItem`
  (returns (Item :type String))
  (`KismetSystemLibrary.PrintString` "Item Get")
  (`self.Destroy item`)
  (return (`self.Item`)))

(fn `UserConstructionScript`)
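; BP_TV_NEW is a TV actor that plays a video once a VHS tape is inserted.
; A trigger shows a key prompt widget while the third-person character overlaps it, skipping creation if a tape is already in.
; InsertTape, which nothing in this graph calls, sets the inserted flag, removes the prompt and calls PlayVideo.
; PlayVideo swaps the screen material from its idle one to M_TV and opens a fixed file media source.
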(event `self.ReceiveBeginPlay`
  (`PrimitiveComponent.SetMaterial` (`self.TVMesh`) 4 "/Game/BPs/Monster/Monster2/aiStandardSurface19.aiStandardSurface19"))

(event `self.trigger.OnComponentBeginOverlap`
  (params (OverlappedComponent :type "PrimitiveComponent Object Reference") (OtherActor :type "Actor Object Reference") (OtherComp :type "PrimitiveComponent Object Reference") (OtherBodyIndex :type Integer) (bFromSweep :type Boolean) (SweepResult :type "HitResult Structure (by ref)"))
  (if (not (`self.TapeInserted`))
    (cast `/Game/ThirdPerson/Blueprints/BP_ThirdPersonCharacter` OtherActor)
    (bind _returnvalue (`|CreateWidget` "/Game/BPs/BP_DisplayKey.BP_DisplayKey_C"))
    (bind _output_get (set `self.KeyPrompt` _returnvalue))
    (`UserWidget.AddToViewport` _output_get 0)))

(event `self.trigger.OnComponentEndOverlap`
  (params (OverlappedComponent :type "PrimitiveComponent Object Reference") (OtherActor :type "Actor Object Reference") (OtherComp :type "PrimitiveComponent Object Reference") (OtherBodyIndex :type Integer))
  (cast `/Game/ThirdPerson/Blueprints/BP_ThirdPersonCharacter` OtherActor)
  (`Widget.RemoveFromParent` (`self.KeyPrompt`)))

(event `PlayVideo`
  (`PrimitiveComponent.SetMaterial` (`self.TVMesh`) 4 "/Game/Movies/M_TV.M_TV")
  (`MediaPlayer.OpenSource` (`self.TVMediaPlayer`) "/Game/Movies/FMS_tape_2.FMS_tape_2"))

(fn `InsertTape`
  (set `self.TapeInserted` true)
  (`KismetSystemLibrary.PrintText` "Inserted VHS into TV!")
  (`self.PlayVideo`)
  (`Widget.RemoveFromParent` (`self.KeyPrompt`)))

(fn `UserConstructionScript`)
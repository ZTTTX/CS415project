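; Monster TV that shows a UI widget while the player is inside its zone and fires a jumpscare once activated.
; ActivateSelf, not called here, swaps the display to its active version, disables collision and sets Active.
; Tick then runs the scare (camera switch, sound, shake, movement disable) and immediately reverts view and movement in the same frame, with no delay.
; Logic to creep toward the player while unseen is unwired.
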(event `self.ReceiveTick`
  (params (DeltaSeconds :type "Float (single-precision)"))
  (if (`self.Active`)
    (`self.jumpScare_TV`)
    (`self.recoverFromJumpScare`)
    (set `self.Active` false)))

(event `self.ActiveZone.OnComponentBeginOverlap`
  (params (OverlappedComponent :type "PrimitiveComponent Object Reference") (OtherActor :type "Actor Object Reference") (OtherComp :type "PrimitiveComponent Object Reference") (OtherBodyIndex :type Integer) (bFromSweep :type Boolean) (SweepResult :type "HitResult Structure (by ref)"))
  (if (not (`self.Active`))
    (cast `/Game/ThirdPerson/Blueprints/BP_ThirdPersonCharacter` OtherActor)
    (bind _returnvalue (`|CreateWidget` "/Game/BPs/Monster/Monster2/BP_Monster2UI.BP_Monster2UI_C"))
    (bind _output_get (set `self.KeyUI` _returnvalue))
    (`UserWidget.AddToViewport` _output_get 0)))

(event `self.ActiveZone.OnComponentEndOverlap`
  (params (OverlappedComponent :type "PrimitiveComponent Object Reference") (OtherActor :type "Actor Object Reference") (OtherComp :type "PrimitiveComponent Object Reference") (OtherBodyIndex :type Integer))
  (cast `/Game/ThirdPerson/Blueprints/BP_ThirdPersonCharacter` OtherActor)
  (`Widget.RemoveFromParent` (`self.KeyUI`)))

(fn `ActivateSelf`
  (set `self.Active` true)
  (`self.SetActorEnableCollision` false)
  (`SceneComponent.SetVisibility` (`self.Display`) false false)
  (`SceneComponent.SetVisibility` (`self.DisplayActive`) true false)
  (`KismetSystemLibrary.PrintText` "ł₦₴ɆⱤ₮ɆĐ VⱧ₴ ł₦₮Ø ₮V!"))

(fn `jumpScare_TV`
  (`ActorComponent.SetActive` (`self.Camera`) true false)
  (`GameplayStatics.PlaySound2D` "/Game/SFX/jumpscare.jumpscare" 4.0 1.0 0.5 null null)
  (`PlayerController.SetViewTargetWithBlend` (`GameplayStatics.GetPlayerController` 0) self 0.01 "VTBlend_Linear" 0.0 false)
  (`GameplayStatics.PlayWorldCameraShake` "/Game/BPs/Monster/BP_cameraShake.BP_cameraShake_C" (`self.K2_GetActorLocation`) 0.0 5000.0)
  (`CharacterMovementComponent.DisableMovement` (`self.CharacterMovement`)))

(fn `recoverFromJumpScare`
  (`PlayerController.SetViewTargetWithBlend` (`GameplayStatics.GetPlayerController` 0) (`GameplayStatics.GetPlayerCharacter` 0) 0.01 "VTBlend_Linear" 0.0 false)
  (`CharacterMovementComponent.SetMovementMode` (`self.CharacterMovement`) "MOVE_Walking" 0)
  (`ActorComponent.SetActive` (`self.Camera`) false false))

(fn `UserConstructionScript`)
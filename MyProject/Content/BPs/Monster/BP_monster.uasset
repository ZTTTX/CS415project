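; Monster AI that roams to random reachable points and chases the player on sight, with chase music that fades after a short roam.
; An AIState enum, dispatched by CheckState, drives AIMoveTo loops for roaming and chasing; hiding players send it back to roam.
; Touching an exposed player applies damage and, if they are alive, triggers a jump scare with sound, camera switch, shake and frozen movement, then restores view and movement.
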(event `self.ReceiveTick`
  (params (DeltaSeconds :type "Float (single-precision)"))
  ;[1 1 1] when stay in Roam for more than 3 sec, fade out the music
  (if (`|EnumEquality` (`self.AIState`) "NewEnumerator1")
    (bind _output_get (set `self.timeInRoam` (+ (`self.timeInRoam`) DeltaSeconds)))
    (if (>= _output_get 2.0)
      (`AudioComponent.FadeOut` (`self.chase`) 2.0 0.0 "Linear"))))

(event `self.ReceiveBeginPlay`
  (set `self.AIState` "NewEnumerator1")
  (`self.CheckState`))

(event `Roam`
  ;[1 1 1] Roaming
  (switch `/Game/BPs/Monster/AIEnum1` (`self.AIState`)
    (:`NewEnumerator1`
      (`KismetSystemLibrary.PrintString` "roaming")
      (`|AIMoveTo` self (`NavigationSystemV1.K2_GetRandomReachablePointInRadius` (`self.K2_GetActorLocation`) 500.0 null null) null
        (:`OnSuccess`
          (`KismetSystemLibrary.PrintString` "SUCESSFULMOVE")
          (`KismetSystemLibrary.Delay` 1.0)
          (`self.CheckState`))))))

(event `ChasePlayer`
  (bind _returnvalue (`GameplayStatics.GetPlayerCharacter` 0))
  ;[1 1 1] Chase
  (`KismetSystemLibrary.PrintString` "chasing player")
  (`|AIMoveTo` self (0.0 0.0 0.0) _returnvalue 3.0
    (:`OnSuccess`
      (bind _asbp_third_person_character (cast `/Game/ThirdPerson/Blueprints/BP_ThirdPersonCharacter` _returnvalue))
      (if (`/Game/ThirdPerson/Blueprints/BP_ThirdPersonCharacter.IsHiding` _asbp_third_person_character)
        (set `self.AIState` "NewEnumerator1")
        (`self.CheckState`)
        (else
          (`KismetSystemLibrary.Delay` 0.2)
          (`self.ChasePlayer`))))
    (:`OnFail`
      (`KismetSystemLibrary.PrintString` "Chase failed." false)
      (set `self.timeInRoam` 0.0)
      (set `self.AIState` "NewEnumerator1")
      (`self.CheckState`))))

(event `self.Sensing1.OnSeePawn`
  (params (Pawn :type "Pawn Object Reference"))
  (bind _chase (`self.chase`))
  ;[1 1 1] switch to chase
  (`KismetSystemLibrary.PrintString` "i see you now" false)
  (bind _asbp_third_person_character (cast `/Game/ThirdPerson/Blueprints/BP_ThirdPersonCharacter` Pawn))
  (if (`/Game/ThirdPerson/Blueprints/BP_ThirdPersonCharacter.IsHiding` _asbp_third_person_character)
    (set `self.AIState` "NewEnumerator1")
    (`self.CheckState`)
    (else
      (`|ExecutionSequence`
        (:`then_0`
          (set `self.AIState` "NewEnumerator2")
          (`self.CheckState`))
        (:`then_1`
          (if (and (not (`AudioComponent.IsPlaying` _chase)) (not (`/Game/ThirdPerson/Blueprints/BP_ThirdPersonCharacter.IsDead` _asbp_third_person_character)))
            (`AudioComponent.Play` _chase 0.0)))))))

(event `CheckState`
  (switch `/Game/BPs/Monster/AIEnum1` (`self.AIState`)
    (:`NewEnumerator1`
      (`self.Roam`))
    (:`NewEnumerator2`
      (`self.ChasePlayer`))))

(event `self.Damage.OnComponentBeginOverlap`
  (params (OverlappedComponent :type "PrimitiveComponent Object Reference") (OtherActor :type "Actor Object Reference") (OtherComp :type "PrimitiveComponent Object Reference") (OtherBodyIndex :type Integer) (bFromSweep :type Boolean) (SweepResult :type "HitResult Structure (by ref)"))
  ;[1 1 1] damage check and jump scare
  (bind _asbp_third_person_character (cast `/Game/ThirdPerson/Blueprints/BP_ThirdPersonCharacter` OtherActor))
  (if (`/Game/ThirdPerson/Blueprints/BP_ThirdPersonCharacter.IsHiding` _asbp_third_person_character)
    (set `self.AIState` "NewEnumerator1")
    (`self.CheckState`)
    (else
      (`|ExecutionSequence`
        (:`then_0`
          (if (not (`/Game/ThirdPerson/Blueprints/BP_ThirdPersonCharacter.IsDead` _asbp_third_person_character))
            (`AudioComponent.Stop` (`self.chase`))
            (`self.jumpScare`)
            (`KismetSystemLibrary.Delay` 3.0)
            (`self.recoverFromJumpScare`)))
        (:`then_1`
          (`GameplayStatics.ApplyDamage` (`GameplayStatics.GetPlayerCharacter` 0) 150.0 null self)
          (`KismetSystemLibrary.Delay` 0.02))))))

(fn `jumpScare`
  (`GameplayStatics.PlaySound2D` "/Game/SFX/jumpscare.jumpscare" 4.0 1.0 0.5 null null)
  (`PlayerController.SetViewTargetWithBlend` (`GameplayStatics.GetPlayerController` 0) self 0.01 "VTBlend_Linear" 0.0 false)
  (`GameplayStatics.PlayWorldCameraShake` "/Game/BPs/Monster/BP_cameraShake.BP_cameraShake_C" (`self.K2_GetActorLocation`) 0.0 5000.0)
  (`CharacterMovementComponent.DisableMovement` (`self.CharacterMovement`)))

(fn `recoverFromJumpScare`
  (`KismetSystemLibrary.PrintString` "Reset camera to player")
  (`PlayerController.SetViewTargetWithBlend` (`GameplayStatics.GetPlayerController` 0) (`GameplayStatics.GetPlayerCharacter` 0) 0.01 "VTBlend_Linear" 0.0 false)
  (`CharacterMovementComponent.SetMovementMode` (`self.CharacterMovement`) "MOVE_Walking" 0))

(fn `UserConstructionScript`)
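; Locker actor that the player can hide in and leave again through the HidePlayer event.
; HidePlayer stores the player, flips the hiding state and replays the door timeline, which drives the door's yaw.
; Hiding makes the player actor invisible and blends the first player controller's view to the locker; leaving reveals the player and blends the view back.
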(event `AnimateDoor`
  (bind (_direction _doortrack) (`Timeline|ToggleDoor` :!via `PlayFromStart`)
    (:`Update`
      (`SceneComponent.K2_SetRelativeRotation` (`self.Door`) (`KismetMathLibrary.MakeRotator` 0.0 0.0 (`KismetMathLibrary.Lerp` 0.0 90.0 _doortrack)) false false))))

(event `HidePlayer`
  (params (Player :type "/Game/ThirdPerson/Blueprints/BP_ThirdPersonCharacter Object Reference"))
  (set `self.PlayerRef` Player)
  (`|ExecutionSequence`
    (:`then_0`
      (`self.ToggleHide`))
    (:`then_1`
      (`self.AnimateDoor`))))

(fn `ToggleHide`
  (bind _returnvalue (`GameplayStatics.GetPlayerController` 0))
  (bind _playerref (`self.PlayerRef`))
  (if (`self.IsHiding`)
    (set `self.IsHiding` false)
    (`self.SetActorHiddenInGame` _playerref false)
    (`PlayerController.SetViewTargetWithBlend` _returnvalue _playerref 0.5 "VTBlend_Linear" 0.0 false)
    (else
      (set `self.IsHiding` true)
      (`self.SetActorHiddenInGame` _playerref true)
      (`PlayerController.SetViewTargetWithBlend` _returnvalue self 0.5 "VTBlend_Linear" 0.0 false))))

(fn `UserConstructionScript`)